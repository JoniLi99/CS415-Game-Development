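; An AI drone that patrols linked PatrolPoints and explodes when destroyed or when its mesh overlaps something.
; Patrol loops AI moves along each point's NextPoint with a one-second delay, while Tick rotates the drone toward its current goal.
; Damage events and collision overlaps reduce health; a surviving drone redirects to the overlapping Pistol, though the failed-cast branch also passes that cast result.
; Explode plays sound and particles, then destroys the actor.
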(event `MoveToTarget`
  (params (NewGoalActor :type "Actor Object Reference (by ref)"))
  (bind _output_get (set `self.GoalActor` NewGoalActor))
  (`|AIMoveTo` self (0.0 0.0 0.0) _output_get))

(event `self.ReceiveBeginPlay`
  (add `self.OnTakeAnyDamage` (delegate `OnTakeDamage`))
  (`self.Patrol`))

(event `OnTakeDamage` :!signature `self.OnTakeAnyDamage`
  (params (DamagedActor :type "Actor Object Reference") (Damage :type "Float (single-precision)") (DamageType :type "DamageType Object Reference") (InstigatedBy :type "Controller Object Reference") (DamageCauser :type "Actor Object Reference"))
  (bind _output_get (set `self.Health` (- (`self.Health`) Damage)))
  (if (<= _output_get 0.0)
    (`self.Explode`)))

(event `self.DroneMesh.OnComponentBeginOverlap`
  (params (OverlappedComponent :type "PrimitiveComponent Object Reference") (OtherActor :type "Actor Object Reference") (OtherComp :type "PrimitiveComponent Object Reference") (OtherBodyIndex :type Integer) (bFromSweep :type Boolean) (SweepResult :type "HitResult Structure (by ref)"))
  (`KismetSystemLibrary.PrintString` "BOOM")
  (`self.Explode`))

(event `self.DroneCollision.OnComponentBeginOverlap`
  (params (OverlappedComponent :type "PrimitiveComponent Object Reference") (OtherActor :type "Actor Object Reference") (OtherComp :type "PrimitiveComponent Object Reference") (OtherBodyIndex :type Integer) (bFromSweep :type Boolean) (SweepResult :type "HitResult Structure (by ref)"))
  (bind _output_get (set `self.Health` (- (`self.Health`) 1.0)))
  (if (<= _output_get 0.0)
    (`self.Explode`)
    (else
      (bind _aspistol (cast `/Game/VRTemplate/Blueprints/Pistol` OtherActor)
        (:`then`
          (`/Engine/EditorBlueprintResources/StandardMacros.IsValid` self
            (:`Is Valid`
              (`self.MoveToTarget` _aspistol))))
        (:`CastFailed`
          (`/Engine/EditorBlueprintResources/StandardMacros.IsValid` self
            (:`Is Valid`
              (`self.MoveToTarget` _aspistol))))))))

(event `self.ReceiveTick`
  (params (DeltaSeconds :type "Float (single-precision)"))
  (bind _goalactor (`self.GoalActor`))
  (`/Engine/EditorBlueprintResources/StandardMacros.IsValid` _goalactor
    (:`Is Valid`
      (`self.K2_SetActorRotation` (`KismetMathLibrary.RInterpTo` (`self.K2_GetActorRotation`) (`KismetMathLibrary.FindLookAtRotation` (`self.K2_GetActorLocation`) (`self.K2_GetActorLocation` _goalactor)) DeltaSeconds)))))

(fn `Explode`
  (`GameplayStatics.PlaySoundAtLocation` "/Game/StarterContent/Audio/Explosion_Cue.Explosion_Cue" (`self.K2_GetActorLocation`) (struct) 1.0 1.0 0.0 null null null null)
  (`GameplayStatics.SpawnEmitterAtLocation` "/Game/StarterContent/Particles/P_Explosion.P_Explosion" (`self.K2_GetActorLocation`))
  (`self.K2_DestroyActor`))

(fn `UserConstructionScript`)