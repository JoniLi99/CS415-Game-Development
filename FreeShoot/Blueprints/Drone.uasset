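; Explosive drone pawn that patrols linked PatrolPoints and smoothly turns toward its goal actor.
; Patrol loops through AI moves along each point's NextPoint.
; Projectile overlaps on DroneCollision reduce Health; surviving hits trigger MoveToTarget, which flies to a hardcoded location and detonates after a delay.
; Zero health or any DroneMesh overlap calls Explode for sound, particles and destruction; RandomRoam and the damage-event binding are left unwired.
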(event `MoveToTarget`
  (params (`New Goal Actor` :type "Actor Object Reference"))
  (set `self.GoalActor` `New Goal Actor`)
  (`KismetSystemLibrary.PrintString` (`KismetSystemLibrary.GetDisplayName` (`self.PistolPoint`)))
  (`|AIMoveTo` self (-390.0 0.0 80.0) null 90.0
    (:`then`
      (`KismetSystemLibrary.PrintString` "Hello")
      (`KismetSystemLibrary.Delay` 1.5)
      (`GameplayStatics.PlaySoundAtLocation` "/Game/StarterContent/Audio/Explosion_Cue.Explosion_Cue" (-390.0 0.0 80.0) (struct) 1.0 1.0 0.0 null null null null)
      (`GameplayStatics.SpawnEmitterAtLocation` "/Game/StarterContent/Particles/P_Explosion.P_Explosion" (-390.0 0.0 80.0))
      (`self.K2_DestroyActor`))))

(event `self.ReceiveBeginPlay`
  (`KismetSystemLibrary.Delay` 0.1)
  (`KismetSystemLibrary.PrintString` (`KismetSystemLibrary.GetDisplayName` (`self.GoalActor`)))
  (`self.Patrol`))

(event `OnTakeDamage`
  (params (DamagedActor :type "Actor Object Reference") (Damage :type "Float (single-precision)") (DamageType :type "DamageType Object Reference") (InstigatedBy :type "Controller Object Reference") (DamageCauser :type "Actor Object Reference"))
  (bind _output_get (set `self.Health` (- (`self.Health`) Damage)))
  (if (<= _output_get 0.0)
    (`self.Explode`)))

(event `Random Roam`
  (`|AIMoveTo` self (-220.0 280.0 130.0) null 1000.0
    (:`then`
      (`|AIMoveTo` self (-540.0 50.0 140.0) null 1000.0
        (:`then`
          (`|AIMoveTo` self (310.0 -310.0 110.0) null 1000.0))))))

(event `self.DroneCollision.OnComponentBeginOverlap`
  (params (OverlappedComponent :type "PrimitiveComponent Object Reference") (OtherActor :type "Actor Object Reference") (OtherComp :type "PrimitiveComponent Object Reference") (OtherBodyIndex :type Integer) (bFromSweep :type Boolean) (SweepResult :type "HitResult Structure (by ref)"))
  (cast `/Game/VRTemplate/Blueprints/Projectile` OtherActor)
  (bind _output_get (set `self.Health` (- (`self.Health`) 1.0)))
  (`KismetSystemLibrary.PrintString` (`KismetStringLibrary.Conv_DoubleToString` _output_get))
  (if (<= _output_get 0.0)
    (`self.Explode`)
    (else
      (bind _aspistol (cast `/Game/VRTemplate/Blueprints/Pistol` OtherActor)
        (:`then`
          _)
        (:`CastFailed`
          _))
      (`/Engine/EditorBlueprintResources/StandardMacros.IsValid` self
        (:`Is Valid`
          _)
        (:`Is Not Valid`
          _))
      (`self.MoveToTarget` _aspistol))))

(event `self.ReceiveTick`
  (params (DeltaSeconds :type "Float (single-precision)"))
  (bind _goalactor (`self.GoalActor`))
  (`/Engine/EditorBlueprintResources/StandardMacros.IsValid` _goalactor
    (:`Is Valid`
      (`self.K2_SetActorRotation` (`KismetMathLibrary.RInterpTo` (`self.K2_GetActorRotation`) (`KismetMathLibrary.FindLookAtRotation` (`self.K2_GetActorLocation`) (`self.K2_GetActorLocation` _goalactor)) DeltaSeconds)))))

(event `self.DroneMesh.OnComponentBeginOverlap`
  (params (OverlappedComponent :type "PrimitiveComponent Object Reference") (OtherActor :type "Actor Object Reference") (OtherComp :type "PrimitiveComponent Object Reference") (OtherBodyIndex :type Integer) (bFromSweep :type Boolean) (SweepResult :type "HitResult Structure (by ref)"))
  (`KismetSystemLibrary.PrintString` "BOOM")
  (`self.Explode`))

(fn `Explode`
  (`GameplayStatics.PlaySoundAtLocation` "/Game/StarterContent/Audio/Explosion_Cue.Explosion_Cue" (`self.K2_GetActorLocation`) (struct) 1.0 1.0 0.0 null null null null)
  (`GameplayStatics.SpawnEmitterAtLocation` "/Game/StarterContent/Particles/P_Explosion.P_Explosion" (`self.K2_GetActorLocation`))
  (`self.K2_DestroyActor`))

(fn `UserConstructionScript`)